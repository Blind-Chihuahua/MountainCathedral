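; Test actor that visualises a playing sound from pre-analysed loudness, onset and constant-Q frequency data.
; The construction script lays out one instanced mesh per frequency band and finds the peak constant-Q level across channel 0 onsets for normalisation.
; Playback-percent callbacks convert progress to seconds, scale left/right spheres by channel loudness with debug labels, then after a short delay batch-update instance heights from the remapped channel 0 spectrum.
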(event `self.ReceiveBeginPlay`
  (bind _inputaudio (`self.InputAudio`))
  (`StaticMeshComponent.SetStaticMesh` (`self.InstancedStaticMesh`) (`self.StaticMeshToSet`))
  (`AudioComponent.SetSound` _inputaudio (`self.SoundWaveToAnalyse`))
  (add `AudioComponent.OnAudioPlaybackPercent` (`self.InputAudio`) (delegate `OnAudioPlaybackPercent_Event`))
  (`AudioComponent.Play` _inputaudio 0.0))

(event `OnAudioPlaybackPercent_Event`
  (params (PlayingSoundWave :type "SoundWave Object Reference") (PlaybackPercent :type "Float (single-precision)"))
  (bind _returnvalue (* PlaybackPercent (`self.Duration`)))
  (bind _outloudness (`LoudnessNRT.GetNormalizedChannelLoudnessAtTime` (`self.LoudnessAnalyser`) _returnvalue 1))
  (bind _outloudness_2 (`LoudnessNRT.GetNormalizedChannelLoudnessAtTime` (`self.LoudnessAnalyser`) _returnvalue 0))
  (`SceneComponent.SetRelativeScale3D` (`self.SM_Sphere_L`) (`KismetMathLibrary.Conv_DoubleToVector` _outloudness_2))
  (`/Game/Blueprint/UtilitiesFunctions/BPF_StringUtilities.Print Label` "L" (`self.NewMacro` _outloudness_2))
  (`SceneComponent.SetRelativeScale3D` (`self.SM_Sphere_R`) (`KismetMathLibrary.Conv_DoubleToVector` _outloudness))
  (`/Game/Blueprint/UtilitiesFunctions/BPF_StringUtilities.Print Label` "R" (`self.NewMacro` _outloudness))
  (`KismetSystemLibrary.Delay` 0.05)
  (`self.UpdateInstances` _returnvalue 15.0))

(fn `RemapFreqResponse`
  (params (Array :type "Array of Float (single-precision)") (InRangeA :type "Float (double-precision)") (InRangeB :type "Float (double-precision)"))
  (returns (Output_Get :type "Array of Float (single-precision)"))
  (locals (NewLocalVar_3 :type "Array of Float (double-precision)"))
  (bind _newlocalvar_3 (`local.NewLocalVar_3`))
  (for _array_element Array
    (`KismetArrayLibrary.Array_Add` _newlocalvar_3 (`KismetMathLibrary.MapRangeClamped` _array_element InRangeA InRangeB 0.0 1.0)))
  (return _newlocalvar_3))

(fn `Setup Instances`
  (params (Spacing :type Integer))
  (for _index (range (+ (`ConstantQNRTSettings.NumBands` (`ConstantQNRT.Settings` (`self.FreqAnalyser`))) 1))
    (`InstancedStaticMeshComponent.AddInstance` (`self.InstancedStaticMesh`) (`KismetMathLibrary.MakeTransform` (`KismetMathLibrary.MakeVector` (`KismetMathLibrary.Conv_IntToDouble` (* _index Spacing)))) false))
  (return))

(fn `UpdateInstances`
  (params (InSeconds :type "Float (single-precision)") (`Height Scale` :type "Float (double-precision)"))
  (returns (Success :type Boolean))
  (locals (NewLocalVar_2 :type "Array of Transform Structure"))
  (bind _output_get (`self.RemapFreqResponse` (`ConstantQNRT.GetChannelConstantQAtTime` (`self.FreqAnalyser`) InSeconds 0) -60.0 (`self.FreqMax`)))
  (for _index (range (`InstancedStaticMeshComponent.GetInstanceCount` (`self.InstancedStaticMesh`)))
    (`KismetArrayLibrary.Array_Add` (`local.NewLocalVar_2`) (`KismetMathLibrary.MakeTransform` (.location (`InstancedStaticMeshComponent.GetInstanceTransform` (`self.InstancedStaticMesh`) _index false)) (struct) (`KismetMathLibrary.MakeVector` 1.0 1.0 (/ (`KismetMathLibrary.FMax` (* (`|GetArrayItem` _output_get _index) `Height Scale`) 2.0) (`self.ScaleToDivideBy`))))))
  (bind _returnvalue (`InstancedStaticMeshComponent.BatchUpdateInstancesTransforms` (`self.InstancedStaticMesh`) 0 (`local.NewLocalVar_2`) false true false))
  (return _returnvalue))

(fn `UserConstructionScript`
  (locals (NewLocalVar :type "Array of Float (single-precision)") (NewLocalVar_0 :type "Array of Float (double-precision)") (NewLocalVar_1 :type "Float (single-precision)" :default 0.0))
  (bind _sound (`AudioAnalyzerNRT.Sound` (`self.LoudnessAnalyser`)))
  (bind _duration (`SoundBase.Duration` _sound))
  (bind _outonsettimestamps (`OnsetNRT.GetChannelOnsetsBetweenTimes` (`self.EventAnalyser`) 0.0 _duration 0))
  (`self.Setup Instances` 150)
  (`AudioComponent.SetSound` (`self.InputAudio`) _sound)
  (set `self.Duration` _duration)
  (set `self.Out Onset Timestamps` _outonsettimestamps)
  (bind _output_get (`self.GetFreqMax` _outonsettimestamps (`self.FreqAnalyser`))
    (:`Completed`
      (bind _output_get_2 (set `self.FreqMax` _output_get))
      (bind _output_get_3 (`self.RemapFreqResponse` (`ConstantQNRT.GetChannelConstantQAtTime` (`self.FreqAnalyser`) (`self.FreqTimeStamp`) 0) -60.0 _output_get_2))
      (set `self.Out Constant Q` _output_get_3))))